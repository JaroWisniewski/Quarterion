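; Enemy Grey character with separate health for each arm and leg, driving injury states, animation and movement.
; Each Tick, CheckHealth grades and regenerates limbs, then priority functions track the worse side to select animation states and leg-based speed, acceleration and jump.
; IsPatrolling runs last, overriding injury movement in one AI state.
; Heavy arm injury drops combat mode, which an input action toggles; limb health displays start hidden.
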(event EventTick
  (params (DeltaSeconds :type Float%20%28single-precision%29))
  (CallFunction|CheckHealth)
  (CallFunction|LegPriority)
  (CallFunction|ArmPriority)
  (CallFunction|SetLegAnimationState)
  (CallFunction|SetArmAnimationState)
  (CallFunction|ChangeVelocity)
  (CallFunction|IsPatrolling?))

(event EventBeginPlay
  (Rendering|SetVisibility (Variables|Default|GetHealth%20Left%20Leg) false false)
  (Rendering|SetVisibility (Variables|Default|GetHealth%20Right%20Leg) false false)
  (Rendering|SetVisibility (Variables|Default|GetHealth%20Left%20Arm) false false)
  (Rendering|SetVisibility (Variables|Default|GetHealth%20Right%20Arm) false false)
  (Rendering|SetVisibility (Variables|Default|GetHealth%20Left%20Arm%20Front) false false)
  (Rendering|SetVisibility (Variables|Default|GetHealth%20Right%20Arm%20Front) false false)
  (Rendering|SetVisibility (Variables|Default|GetHealth%20Left%20Leg%20Front) false false)
  (Rendering|SetVisibility (Variables|Default|GetHealth%20Right%20Leg%20Front) false false))

(event Input|ActionEvents|InputActionCombatMode
  (params (Key :type Key%20Structure))
  (:Pressed
    ;[1 1 1] Equip Weapon
    (if (Variables|Default|GetCombat)
      (Variables|Default|SetCombat false)
      (Variables|Default|SetEquipped false)
      (else
        (Variables|Default|SetCombat true)
        (Utilities|FlowControl|Delay 0.3)
        (Variables|Default|SetEquipped true)))))

(fn ConstructionScript)

(fn CheckHealth
  ;[1 1 1] Setting the Left Leg Health State
  (if (<= (Variables|Health|GetLeftLegHealth) 7e+01)
    (if (< (Variables|Health|GetLeftLegHealth) 4e+01)
      (Variables|Health|SetLeftLegHealthState "NewEnumerator2")
      (Variables|Health|SetLeftLegDamage 2)
      (if (< (Variables|Health|GetLeftLegHealth) 15.0)
        (Variables|Health|SetLeftLegHealthState "NewEnumerator3")
        (Variables|Health|SetLeftLegDamage 3))
      (else
        (Variables|Health|SetLeftLegHealthState "NewEnumerator1")
        (Variables|Health|SetLeftLegDamage 1)))
    (else
      (Variables|Health|SetLeftLegHealthState "NewEnumerator0")
      (Variables|Health|SetLeftLegDamage 0)))
  ;[1 1 1] Setting the Right Leg Health State
  (if (<= (Variables|Health|GetRightLegHealth) 7e+01)
    (if (< (Variables|Health|GetRightLegHealth) 4e+01)
      (Variables|Health|SetRightLegHealthState "NewEnumerator2")
      (Variables|Health|SetRightLegDamage 2)
      (if (< (Variables|Health|GetRightLegHealth) 15.0)
        (Variables|Health|SetRightLegHealthState "NewEnumerator3")
        (Variables|Health|SetRightLegDamage 3))
      (else
        (Variables|Health|SetRightLegHealthState "NewEnumerator1")
        (Variables|Health|SetRightLegDamage 1)))
    (else
      (Variables|Health|SetRightLegHealthState "NewEnumerator0")
      (Variables|Health|SetRightLegDamage 0)))
  ;[1 1 1] Setting the Right Arm Health State
  (if (<= (Variables|Health|GetRightArmHealth) 7e+01)
    (if (< (Variables|Health|GetRightArmHealth) 4e+01)
      (Variables|Health|SetRightArmHealthState "NewEnumerator2")
      (Variables|Health|SetRightArmDamage 2)
      (if (< (Variables|Health|GetRightArmHealth) 15.0)
        (Variables|Health|SetRightArmHealthState "NewEnumerator3")
        (Variables|Health|SetRightArmDamage 3)
        ;;[1 1 1] Drop Weapon
        (Variables|Default|SetCombat false)
        (Variables|Default|SetEquipped false))
      (else
        (Variables|Health|SetRightArmHealthState "NewEnumerator1")
        (Variables|Health|SetRightArmDamage 1)))
    (else
      (Variables|Health|SetRightArmHealthState "NewEnumerator0")
      (Variables|Health|SetRightArmDamage 0)))
  ;[1 1 1] Setting the Left Arm Health State
  (if (<= (Variables|Health|GetLeftArmHealth) 7e+01)
    (if (< (Variables|Health|GetLeftArmHealth) 4e+01)
      (Variables|Health|SetLeftArmHealthState "NewEnumerator2")
      (Variables|Health|SetLeftArmDamage 2)
      (if (< (Variables|Health|GetLeftArmHealth) 15.0)
        (Variables|Health|SetLeftArmHealthState "NewEnumerator3")
        (Variables|Health|SetLeftArmDamage 3)
        ;;[1 1 1] Drop Weapon
        (Variables|Default|SetCombat false)
        (Variables|Default|SetEquipped false))
      (else
        (Variables|Health|SetLeftArmHealthState "NewEnumerator1")
        (Variables|Health|SetLeftArmDamage 1)))
    (else
      (Variables|Health|SetLeftArmHealthState "NewEnumerator0")
      (Variables|Health|SetLeftArmDamage 0)))
  (if false
    _
    (else
      _))
  (if (< (Variables|Health|GetLeftLegHealth) (Variables|Health|GetMaxHealth))
    ;[1 1 1] Left Leg Regeneration
    (Variables|Health|SetLeftLegHealth (+ (Variables|Health|GetLeftLegHealth) (* (Utilities|Time|GetWorldDeltaSeconds) 1.0))))
  (if (< (Variables|Health|GetRightLegHealth) (Variables|Health|GetMaxHealth))
    ;[1 1 1] Right Leg Regeneration
    (Variables|Health|SetRightLegHealth (+ (Variables|Health|GetRightLegHealth) (* (Utilities|Time|GetWorldDeltaSeconds) 1.0))))
  (if (< (Variables|Health|GetRightArmHealth) (Variables|Health|GetMaxHealth))
    ;[1 1 1] Right Arm Regeneration
    (Variables|Health|SetRightArmHealth (+ (Variables|Health|GetRightArmHealth) (* (Utilities|Time|GetWorldDeltaSeconds) 1.0))))
  (if (< (Variables|Health|GetLeftArmHealth) (Variables|Health|GetMaxHealth))
    ;[1 1 1] Left Arm Regeneration
    (Variables|Health|SetLeftArmHealth (+ (Variables|Health|GetLeftArmHealth) (* (Utilities|Time|GetWorldDeltaSeconds) 1.0)))))

(fn ChangeVelocity
  (bind _charactermovement (Variables|Character|GetCharacterMovement))
  (if (Variables|Default|GetLeftLegDamagePriority)
    (switch Utilities|FlowControl|Switch|SwitchonLeftLegHealthState (Variables|Health|GetLeftLegHealthState)
      (:NewEnumerator0
        (Variables|/Script/Engine.CharacterMovementComponent|SetMaxAcceleration _charactermovement 2048.0 :!label _label)
        (Variables|/Script/Engine.CharacterMovementComponent|SetMaxWalkSpeed _charactermovement 6e+02)
        (Variables|/Script/Engine.CharacterMovementComponent|SetJumpZVelocity _charactermovement 6e+02))
      (:NewEnumerator1
        (Variables|/Script/Engine.CharacterMovementComponent|SetMaxAcceleration _charactermovement 2048.0 :!label _label_2)
        (Variables|/Script/Engine.CharacterMovementComponent|SetMaxWalkSpeed _charactermovement 4.5e+02)
        (Variables|/Script/Engine.CharacterMovementComponent|SetJumpZVelocity _charactermovement 6e+02))
      (:NewEnumerator2
        (Variables|/Script/Engine.CharacterMovementComponent|SetMaxAcceleration _charactermovement 1024.0 :!label _label_3)
        (Variables|/Script/Engine.CharacterMovementComponent|SetMaxWalkSpeed _charactermovement 2e+02)
        (Variables|/Script/Engine.CharacterMovementComponent|SetJumpZVelocity _charactermovement 4e+02))
      (:NewEnumerator3
        (Variables|/Script/Engine.CharacterMovementComponent|SetMaxAcceleration _charactermovement 6e+02 :!label _label_4)
        (Variables|/Script/Engine.CharacterMovementComponent|SetMaxWalkSpeed _charactermovement 1e+02)
        (Variables|/Script/Engine.CharacterMovementComponent|SetJumpZVelocity _charactermovement 1e+02)))
    (else
      (switch Utilities|FlowControl|Switch|SwitchonRightLegHealthState (Variables|Health|GetRightLegHealthState)
        (:NewEnumerator0
          (goto _label))
        (:NewEnumerator1
          (goto _label_2))
        (:NewEnumerator2
          (goto _label_3))
        (:NewEnumerator3
          (goto _label_4))))))

(fn LegPriority
  (if (> (Variables|Health|GetLeftLegDamage) (Variables|Health|GetRightLegDamage))
    (Variables|Default|SetLeftLegDamagePriority true)
    (elif (not (== (Variables|Health|GetLeftLegDamage) (Variables|Health|GetRightLegDamage)))
      (Variables|Default|SetLeftLegDamagePriority false))))

(fn SetLegAnimationState
  (if (< (Variables|Health|GetRightLegDamage) (Variables|Health|GetLeftLegDamage))
    (if (< (Variables|Health|GetLeftLegDamage) 2)
      (Variables|Health|SetLegAnimationState "NewEnumerator0")
      (elif (== (Variables|Health|GetLeftLegDamage) 2)
        (Variables|Health|SetLegAnimationState "NewEnumerator1")
        (else
          (Variables|Health|SetLegAnimationState "NewEnumerator2"))))
    (elif (< (Variables|Health|GetRightLegDamage) 2)
      (Variables|Health|SetLegAnimationState "NewEnumerator0")
      (elif (== (Variables|Health|GetRightLegDamage) 2)
        (Variables|Health|SetLegAnimationState "NewEnumerator3")
        (else
          (Variables|Health|SetLegAnimationState "NewEnumerator5"))))))

(fn ArmPriority
  (if (> (Variables|Health|GetLeftArmDamage) (Variables|Health|GetRightArmDamage))
    (Variables|Default|SetLeftArmDamagePriority true)
    (elif (not (== (Variables|Health|GetLeftArmDamage) (Variables|Health|GetRightArmDamage)))
      (Variables|Default|SetLeftArmDamagePriority false))))

(fn SetArmAnimationState
  (if (Variables|Default|GetLeftArmDamagePriority)
    (if (< (Variables|Health|GetLeftArmDamage) 2)
      (Variables|Health|SetArmAnimationState "NewEnumerator0")
      (elif (== (Variables|Health|GetLeftArmDamage) 2)
        (Variables|Health|SetArmAnimationState "NewEnumerator1")
        (else
          (Variables|Health|SetArmAnimationState "NewEnumerator2"))))
    (elif (< (Variables|Health|GetRightArmDamage) 2)
      (Variables|Health|SetArmAnimationState "NewEnumerator0")
      (elif (== (Variables|Health|GetRightArmDamage) 2)
        (Variables|Health|SetArmAnimationState "NewEnumerator3")
        (else
          (Variables|Health|SetArmAnimationState "NewEnumerator5"))))))

(fn IsPatrolling?
  (bind _charactermovement (Variables|Character|GetCharacterMovement))
  (if (Utilities|Enum|Equal(Enum) (Variables|Default|GetAI%20State) "NewEnumerator0")
    (Variables|/Script/Engine.CharacterMovementComponent|SetMaxAcceleration _charactermovement 2048.0)
    (Variables|/Script/Engine.CharacterMovementComponent|SetMaxWalkSpeed _charactermovement 7e+01)
    (Variables|/Script/Engine.CharacterMovementComponent|SetJumpZVelocity _charactermovement 6e+02)))