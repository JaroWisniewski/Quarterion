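; Grey_AI is the AI controller logic for the Grey character, driving its behavior tree and tracking enemies through perception.
; On BeginPlay it sets up the Grey_BBoard blackboard, runs Grey_BTree and keeps the blackboard component.
; AI perception updates write any sensed actor tagged "Dreyar" to the enemy key, and clear that key when such an actor's stimulus is lost.
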(event OnTargetPerceptionUpdated(AIPerception)
  (params (Actor :type Actor%20Object%20Reference) (Stimulus :type AI%20Stimulus%20Structure))
  (bind _enemykey (Variables|Default|GetEnemyKey))
  (bind _blackbboardcomp (Variables|Default|GetBlackbboardComp))
  (if (Actor|ActorHasTag Actor "Dreyar")
    (if (.bsuccessfullysensed Stimulus)
      (AI|Components|Blackboard|SetValueasObject _blackbboardcomp _enemykey Actor)
      (else
        (AI|Components|Blackboard|ClearValue _blackbboardcomp _enemykey)))))

(event EventBeginPlay
  (bind _blackboardcomponent (Class|AIController|UseBlackboard "/Game/Characters/Grey/Blueprints/AI/Grey_BBoard.Grey_BBoard"))
  (AI|RunBehaviorTree "/Game/Characters/Grey/Blueprints/AI/Grey_BTree.Grey_BTree")
  (Variables|Default|SetBlackbboardComp _blackboardcomponent))

(event EventTick
  (params (DeltaSeconds :type Float%20%28single-precision%29)))

(fn ConstructionScript)