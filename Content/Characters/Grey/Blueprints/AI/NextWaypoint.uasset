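; Behavior Tree task for the Grey enemy that advances it to the next waypoint of its patrol route.
; On execute it sets the pawn's AIState, noted as a speed change, and writes the patrol point at the current WaypointIndex to the Waypoint Blackboard key.
; It then increments the index modulo the PatrolPoints count, so the route loops, and finishes successfully.
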(event EventReceiveExecuteAI
  (params (OwnerController :type AI%20Controller%20Object%20Reference) (ControlledPawn :type Pawn%20Object%20Reference))
  (CallFunction|GetPatrolPoints ControlledPawn)
  (bind _index (CallFunction|GetNextWaypoint))
  (CallFunction|IncrementIndex _index)
  (AI|BehaviorTree|FinishExecute true))

(fn GetPatrolPoints
  (params (Owner :type Object%20Object%20Reference))
  (bind _asenemy_grey (Utilities|Casting|CastToEnemyGrey Owner))
  ;[1 1 1] Change Speed
  (Variables|/Game/Characters/Grey/Blueprints/EnemyGrey.EnemyGrey_C|SetAI%20State _asenemy_grey "NewEnumerator0"))

(fn GetNextWaypoint
  (bind _waypointindex (Variables|Default|GetWaypointIndex))
  (bind _returnvalue (Class|BTFunctionLibrary|GetBlackboardValueasInt _waypointindex))
  (Class|BTFunctionLibrary|SetBlackboardValueasObject (Variables|Default|GetWaypoint) (Utilities|Array|Get(acopy) (Variables|Default|GetPatrol%20Points) _returnvalue))
  (return _returnvalue))

(fn IncrementIndex
  (params (Index :type Integer%20%28by%20ref%29))
  (bind _result (Math|Integer|IncrementInt Index)
    (:%20%20
      (Class|BTFunctionLibrary|SetBlackboardValueasInt (Variables|Default|GetWaypointIndex) (Math|Integer|%(Integer) _result (Utilities|Array|Length (Variables|Default|GetPatrol%20Points)))))))